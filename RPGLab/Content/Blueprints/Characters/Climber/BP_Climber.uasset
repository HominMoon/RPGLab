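; BP_Climber is a climber character Blueprint that routes Enhanced Input to movement and ledge actions.
; The jump input performs a normal jump, or while hanging either a side ledge jump or a ledge climb, depending on IsLedgeJumping.
; The move input passes its 2D axis to Move on both Triggered and Completed.
; The movement and ledge logic is called here but not defined in this Blueprint.
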(event Input|EnhancedActionEvents|EnhancedInputActionIA_Jump
  (params (ActionValue :type Boolean) (ElapsedSeconds :type Float%20%28double-precision%29) (TriggeredSeconds :type Float%20%28double-precision%29) (InputAction :type Input%20Action%20Object%20Reference :default "/Game/Blueprints/EnhancedInput/MarkerMan/IA_Jump.IA_Jump"))
  (:Triggered
    (if (Variables|Default|GetbIsHanging)
      (if (Variables|Default|GetbIsLedgeJumping)
        (Class|Climber|JumpSideLedge)
        (else
          (Class|Climber|ClimbLedge)))
      (else
        (Character|Jump)))))

(event Input|EnhancedActionEvents|EnhancedInputActionIA_Markerman_Move
  (params (ActionValue :type Vector%202D%20Structure) (ElapsedSeconds :type Float%20%28double-precision%29) (TriggeredSeconds :type Float%20%28double-precision%29) (InputAction :type Input%20Action%20Object%20Reference :default "/Game/Blueprints/EnhancedInput/MarkerMan/IA_Markerman_Move.IA_Markerman_Move"))
  (:Triggered
    (Class|Climber|Move (Utilities|Struct|MakeInputActionValue (.x ActionValue) (.y ActionValue) 0.0 "Axis2D") :!label _label))
  (:Completed
    (goto _label)))

(event EventBeginPlay)

(event Collision|EventActorBeginOverlap
  (params (OtherActor :type Actor%20Object%20Reference)))

(event EventTick
  (params (DeltaSeconds :type Float%20%28single-precision%29)))

(fn ConstructionScript)